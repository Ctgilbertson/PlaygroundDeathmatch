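; Enemy character Blueprint that handles taking damage and dying.
; The AnyDamage event subtracts damage from Health and starts the death sequence at zero or below.
; Death turns the mesh into a physics ragdoll, disables movement and removes the capsule, then destroys the actor after a random delay of a few seconds.
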(event Game|Damage|EventAnyDamage
  (params (Damage :type Float%20%28single-precision%29) (DamageType :type Damage%20Type%20Object%20Reference) (InstigatedBy :type Controller%20Object%20Reference) (DamageCauser :type Actor%20Object%20Reference))
  ;[1 1 1] Take damage/kill
  (bind _output_get (Variables|Default|SetHealth (- (Variables|Default|GetHealth) Damage)))
  (if (<= _output_get 0.0)
    ;[1 1 1] Ragdoll
    (Physics|SetSimulatePhysics (Variables|Character|GetMesh) true)
    (Pawn|Components|CharacterMovement|DisableMovement (Variables|Character|GetCharacterMovement))
    (Components|DestroyComponent (Variables|Collision|GetCapsuleComponent))
    (Collision|SetCollisionProfileName (Variables|Character|GetMesh) "ragdoll" true :!class /Script/Engine.PrimitiveComponent)
    (Utilities|FlowControl|Delay (Math|Random|RandomFloatinRange 3.0 1e+01))
    (Actor|DestroyActor)))

(fn ConstructionScript)